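; Spawner actor that creates enemy spider bots at its own location in the mech combat game.
; SpawnExplosive spawns a Spider_Bomb and SpawnTourette spawns a Spider_Tourette, both as AI pawns.
; Each function then increments NumberOfBots on the ThirdPersonGameMode to track the bot count.
; It has no active events of its own, so spawning runs only when these functions are called.
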(event EventBeginPlay)

(event Collision|EventActorBeginOverlap
  (params (OtherActor :type Actor%20Object%20Reference)))

(event EventTick
  (params (DeltaSeconds :type Float%20%28single-precision%29)))

(fn ConstructionScript)

(fn SpawnExplosive
  (AI|SpawnAIFromClass "/Game/ThirdPersonBP/Blueprints/Spider_Bomb.Spider_Bomb_C" 0 (Transformation|GetActorLocation) "0, 0, 0" false 0)
  (bind _asthird_person_game_mode (Utilities|Casting|CastToThirdPersonGameMode (Game|GetGameMode)))
  (Math|Integer|IncrementInt (Variables|/Game/ThirdPersonBP/Blueprints/ThirdPersonGameMode.ThirdPersonGameMode_C|GetNumberOfBots _asthird_person_game_mode)))

(fn SpawnTourette
  (AI|SpawnAIFromClass "/Game/ThirdPersonBP/Blueprints/Spider_Tourette.Spider_Tourette_C" 0 (Transformation|GetActorLocation) "0, 0, 0" false 0)
  (bind _asthird_person_game_mode (Utilities|Casting|CastToThirdPersonGameMode (Game|GetGameMode)))
  (Math|Integer|IncrementInt (Variables|/Game/ThirdPersonBP/Blueprints/ThirdPersonGameMode.ThirdPersonGameMode_C|GetNumberOfBots _asthird_person_game_mode)))